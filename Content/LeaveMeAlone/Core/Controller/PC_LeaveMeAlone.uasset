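; Player controller for LeaveMeAlone that handles pause, time-expired and game-over screens and carries player progress through a save slot.
; Each screen pauses the game and shows a UI-only widget with the cursor; the time-expired widget depends on whether the level is FirstLevel.
; Time expiry and game over save health, score and best score, with expiry suppressing later game over.
; BeginPlay restores health and score after a short delay.
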(event Custom|TimeExpiredEvent
  (Variables|Default|SetTimeExpired true)
  (CallFunction|SaveGame)
  (CallFunction|PauseCharacter)
  (Game|SetGamePaused true)
  (bind _returnvalue (Game|GetCurrentLevelName true))
  (if (Utilities|Enum|Equal(Enum) _returnvalue "FirstLevel")
    (bind _returnvalue_2 (UserInterface|CreateWidget "/Game/LeaveMeAlone/Widgets/UI/WBP_TimeExpired_0.WBP_TimeExpired_0_C"))
    (bind _output_get (Variables|Default|SetTimeExpiredWidget_0 _returnvalue_2))
    (UserInterface|Viewport|AddtoViewport _output_get 0)
    (Input|SetInputModeUIOnly self _output_get "DoNotLock" true)
    (else
      (bind _returnvalue_3 (UserInterface|CreateWidget "/Game/LeaveMeAlone/Widgets/UI/WBP_TimeExpired_1.WBP_TimeExpired_1_C"))
      (bind _output_get_2 (Variables|Default|SetTimeExpiredWidget_1 _returnvalue_3))
      (UserInterface|Viewport|AddtoViewport _output_get_2 0)
      (Input|SetInputModeUIOnly self _output_get_2 "DoNotLock" true)))
  (Variables|Default|SetbShowMouseCursor true))

(event Custom|GameOverEvent
  (if (not (Variables|Default|GetTimeExpired))
    (CallFunction|SaveGame)
    (Utilities|FlowControl|Delay 3.0)
    (Game|SetGamePaused true)
    (bind _returnvalue (UserInterface|CreateWidget "/Game/LeaveMeAlone/Widgets/UI/WBP_GameOver.WBP_GameOver_C"))
    (bind _output_get (Variables|Default|SetGameOverWidget _returnvalue))
    (UserInterface|Viewport|AddtoViewport _output_get 0)
    (Input|SetInputModeUIOnly self _output_get "DoNotLock" true)
    (Variables|Default|SetbShowMouseCursor true)))

(event EventBeginPlay
  (Utilities|FlowControl|Delay 0.3)
  (CallFunction|LoadGame))

(event EventTick
  (params (DeltaSeconds :type Float%20%28single-precision%29)))

(event Input|ActionEvents|InputActionPause
  (params (Key :type Key%20Structure :default "None"))
  (:Pressed
    (if (not (Variables|Default|GetOnPause))
      (bind _output_get (Variables|Default|SetOnPause true))
      (CallFunction|PauseCharacter)
      (Game|SetGamePaused _output_get)
      (bind _returnvalue (UserInterface|CreateWidget "/Game/LeaveMeAlone/Widgets/UI/WBP_Pause.WBP_Pause_C"))
      (bind _output_get_2 (Variables|Default|SetPauseWidget _returnvalue))
      (UserInterface|Viewport|AddtoViewport _output_get_2 0)
      (Input|SetInputModeUIOnly self _output_get_2 "DoNotLock" true)
      (Variables|Default|SetbShowMouseCursor true))))

(fn ConstructionScript)

(fn SaveGame
  (bind _returnvalue (SaveGame|DoesSaveGameExist "LMA_SaveGame"))
  (if _returnvalue
    (bind _returnvalue_2 (SaveGame|LoadGamefromSlot "LMA_SaveGame"))
    (bind _assg_parameters (Utilities|Casting|CastToSG_Parameters _returnvalue_2))
    (Variables|Default|SetLevelSaveGame _assg_parameters)
    (else
      (bind _returnvalue_3 (SaveGame|CreateSaveGameObject "/Game/LeaveMeAlone/SaveGame/SG_Parameters.SG_Parameters_C"))
      (bind _output_get (Variables|Default|SetLevelSaveGame _returnvalue_3))
      (Variables|/Game/LeaveMeAlone/SaveGame/SG_Parameters.SG_Parameters_C|SetBestScore _output_get 0)))
  (bind _asch_player (Utilities|Casting|CastToCH_Player (Game|GetPlayerCharacter 0))
    (:then
      (Variables|/Game/LeaveMeAlone/SaveGame/SG_Parameters.SG_Parameters_C|SetCurrentHealth (Variables|Default|GetLevelSaveGame) (Class|LMAHealthComponent|GetHealth (Variables|/Script/LeaveMeAlone.LMADefaultCharacter|GetHealthComponent _asch_player))))
    (:CastFailed
      _))
  (bind _aspc_leave_me_alone (Utilities|Casting|CastToPC_LeaveMeAlone (Game|GetPlayerController 0)))
  (Variables|/Game/LeaveMeAlone/SaveGame/SG_Parameters.SG_Parameters_C|SetCurrentScores (Variables|Default|GetLevelSaveGame) (Variables|PC_LeaveMeAlone_C|GetScore _aspc_leave_me_alone))
  (if (> (Variables|PC_LeaveMeAlone_C|GetScore _aspc_leave_me_alone) (Variables|/Game/LeaveMeAlone/SaveGame/SG_Parameters.SG_Parameters_C|GetBestScore (Variables|Default|GetLevelSaveGame)))
    (Variables|/Game/LeaveMeAlone/SaveGame/SG_Parameters.SG_Parameters_C|SetBestScore (Variables|Default|GetLevelSaveGame) (Variables|PC_LeaveMeAlone_C|GetScore _aspc_leave_me_alone)))
  (SaveGame|SaveGametoSlot (Variables|Default|GetLevelSaveGame) "LMA_SaveGame")
  (return))

(fn LoadGame
  (bind _returnvalue (SaveGame|DoesSaveGameExist "LMA_SaveGame"))
  (if _returnvalue
    (bind _returnvalue_2 (SaveGame|LoadGamefromSlot "LMA_SaveGame"))
    (bind _assg_parameters (Utilities|Casting|CastToSG_Parameters _returnvalue_2))
    (Variables|Default|SetLevelSaveGame _assg_parameters)
    (else
      (bind _returnvalue_3 (SaveGame|CreateSaveGameObject "/Game/LeaveMeAlone/SaveGame/SG_Parameters.SG_Parameters_C"))
      (bind _output_get (Variables|Default|SetLevelSaveGame _returnvalue_3))
      (Variables|/Game/LeaveMeAlone/SaveGame/SG_Parameters.SG_Parameters_C|SetBestScore _output_get 0)))
  (bind _asch_player (Utilities|Casting|CastToCH_Player (Game|GetPlayerCharacter 0)))
  (Class|LMAHealthComponent|SetHealth (Variables|/Script/LeaveMeAlone.LMADefaultCharacter|GetHealthComponent _asch_player) (Variables|/Game/LeaveMeAlone/SaveGame/SG_Parameters.SG_Parameters_C|GetCurrentHealth (Variables|Default|GetLevelSaveGame)))
  (bind _aspc_leave_me_alone (Utilities|Casting|CastToPC_LeaveMeAlone (Game|GetPlayerController 0)))
  (Variables|PC_LeaveMeAlone_C|SetScore _aspc_leave_me_alone (Variables|/Game/LeaveMeAlone/SaveGame/SG_Parameters.SG_Parameters_C|GetCurrentScores (Variables|Default|GetLevelSaveGame)))
  (return))

(fn PauseCharacter
  (bind _aslmadefault_character (Utilities|Casting|CastToLMADefaultCharacter (Game|GetPlayerCharacter 0)))
  (Class|LMADefaultCharacter|PauseCharacter _aslmadefault_character)
  (return))