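; GM_LeaveMeAlone is the game mode for LeaveMeAlone that decides when a match ends.
; A looping one-second timer counts GameTime down and, at zero, clears itself and calls TimeExpiredEvent on PC_LeaveMeAlone.
; After a three-second startup delay, Tick calls GameOverEvent on that controller every frame the player character is not valid.
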(event Custom|OncePerSecondEvent
  (bind _output_get (Variables|Default|SetGameTime (- (Variables|Default|GetGameTime) 1)))
  (if (<= _output_get 0)
    (Utilities|Time|ClearandInvalidateTimerbyHandle (Variables|Default|GetGameTimerHandler))
    (bind _aspc_leave_me_alone (Utilities|Casting|CastToPC_LeaveMeAlone (Game|GetPlayerController 0)))
    (Default|TimeExpiredEvent _aspc_leave_me_alone)))

(event EventBeginPlay
  (bind _returnvalue (Utilities|Time|SetTimerbyEvent (delegate Custom|OncePerSecondEvent) 1.0 true))
  (Variables|Default|SetGameTimerHandler _returnvalue)
  (Utilities|FlowControl|Delay 3.0)
  (Variables|Default|SetStartTick true))

(event EventTick
  (params (DeltaSeconds :type Float%20%28single-precision%29))
  (if (Variables|Default|GetStartTick)
    (Utilities|IsValid (Game|GetPlayerCharacter 0)
      (:Is%20Not%20Valid
        (bind _aspc_leave_me_alone (Utilities|Casting|CastToPC_LeaveMeAlone (Game|GetPlayerController 0)))
        (Default|GameOverEvent _aspc_leave_me_alone)))))

(fn ConstructionScript)