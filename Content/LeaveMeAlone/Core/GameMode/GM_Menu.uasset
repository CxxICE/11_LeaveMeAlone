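; Game mode for the main menu that plays the menu music and prepares the player's save data.
; On BeginPlay it starts the menu sound and runs LoadGame, which loads the LMA_SaveGame slot as SG_Parameters and stores it in LevelSaveGame.
; If no save exists, it creates a new save object with the best score at zero, without writing it to disk.
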(event EventBeginPlay
  (Audio|PlaySound2D "/Game/LeaveMeAlone/Audio/Wave/Menu.Menu" 1.0 1.0 0.0 0 0)
  (CallFunction|LoadGame))

(event EventTick
  (params (DeltaSeconds :type Float%20%28single-precision%29)))

(fn ConstructionScript)

(fn LoadGame
  (bind _returnvalue (SaveGame|DoesSaveGameExist "LMA_SaveGame"))
  (if _returnvalue
    (bind _returnvalue_2 (SaveGame|LoadGamefromSlot "LMA_SaveGame"))
    (bind _assg_parameters (Utilities|Casting|CastToSG_Parameters _returnvalue_2))
    (Variables|Default|SetLevelSaveGame _assg_parameters)
    (else
      (bind _returnvalue_3 (SaveGame|CreateSaveGameObject "/Game/LeaveMeAlone/SaveGame/SG_Parameters.SG_Parameters_C"))
      (bind _output_get (Variables|Default|SetLevelSaveGame _returnvalue_3))
      (Variables|/Game/LeaveMeAlone/SaveGame/SG_Parameters.SG_Parameters_C|SetBestScore _output_get 0)))
  (return))